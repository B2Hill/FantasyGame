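; BP_DefaultActor is a selectable, movable pawn that responds to selection and move commands.
; SelectionChange switches the Cube's overlay material between an outline and a no-outline material based on IsSelected.
; MoveCharacter, only while selected, calls MoveChar, which snaps the target to a grid and issues AIMoveTo.
; MoveChar continues after a fixed delay from issuing the move, without waiting for arrival, and debug prints trace both actions.
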(event `SelectionChange`
  (bind _cube (`self.Cube`))
  (if (`self.IsSelected`)
    (`MeshComponent.SetOverlayMaterial` _cube (`self.OutlineMat`))
    (`KismetSystemLibrary.PrintString` "Overlay On")
    (else
      (`MeshComponent.SetOverlayMaterial` _cube "/Game/Assets/Actors/Material/Mat_Outline_Noner.Mat_Outline_Noner")
      (`KismetSystemLibrary.PrintString` "Overlay Off"))))

(event `MoveCharacter`
  (params (MovementLocation :type "Vector Structure"))
  (if (`self.IsSelected`)
    (`self.MoveChar` MovementLocation
      (:`ExecOut`
        (`KismetSystemLibrary.PrintString` "Move")))))

(fn `UserConstructionScript`)